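; Physics-driven, player-controlled tank pawn using Enhanced Input for movement and steering.
; Every tick, it line-traces from six wheels, pushing the Box body with distance-scaled suspension and acceleration forces on hits while interpolating wheel mesh height.
; Move input is smoothed into acceleration, while turn input applies mass-scaled yaw torque, allowing stationary turning.
; Both also rotate left and right wheel sets to animate the tracks, with opposite signs when turning.
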(event `self.ReceiveBeginPlay`
  ; adds mapping context
  (`EnhancedInputSubsystemInterface.AddMappingContext` (pcsubsystem `EnhancedInputLocalPlayerSubsystem` (`GameplayStatics.GetPlayerController` 0)) "/Game/Tank/IMC_TankMovement.IMC_TankMovement" 0 (struct)))

(event `EnhancedInput|/Game/Tank/IA_Move`
  (params (ActionValue :type "Float (double-precision)") (ElapsedSeconds :type "Float (double-precision)") (TriggeredSeconds :type "Float (double-precision)") (InputAction :type "InputAction Object Reference" :default "/Game/Tank/IA_Move.IA_Move"))
  ; Tank Movement/Acceleration
  (:`Triggered`
    (set `self.AccelerationInput` (`KismetMathLibrary.FInterpTo` (`self.AccelerationInput`) ActionValue (`GameplayStatics.GetWorldDeltaSeconds`) 0.5))))

(event `self.ReceiveTick`
  (params (DeltaSeconds :type "Float (single-precision)"))
  ; Casting the suspension for each wheel
  (`self.Suspension Cast` null)
  (`self.CalculateAcceleration`))

(event `EnhancedInput|/Game/Tank/IA_Turn`
  (params (ActionValue :type "Float (double-precision)") (ElapsedSeconds :type "Float (double-precision)") (TriggeredSeconds :type "Float (double-precision)") (InputAction :type "InputAction Object Reference" :default "/Game/Tank/IA_Turn.IA_Turn"))
  ; Tank Steering includes turning when stationary
  (:`Triggered`
    (`self.Calculate Turning` ActionValue)))

(fn `Calculate Left track`
  (params (`Speed Input` :type "Float (double-precision)"))
  (`SceneComponent.K2_AddLocalRotation` (`self.Wheel ML`) (`KismetMathLibrary.MakeRotator` 0.0 0.0 (/ `Speed Input` 0.1)) false false)
  (`SceneComponent.K2_AddLocalRotation` (`self.Wheel FL`) (`KismetMathLibrary.MakeRotator` 0.0 0.0 (/ `Speed Input` 0.1)) false false)
  (`SceneComponent.K2_AddLocalRotation` (`self.Wheel BL`) (`KismetMathLibrary.MakeRotator` 0.0 0.0 (/ `Speed Input` 0.1)) false false))

(fn `Calculate Right Track`
  (params (`Speed Input` :type "Float (double-precision)"))
  (`SceneComponent.K2_AddLocalRotation` (`self.Wheel FR`) (`KismetMathLibrary.MakeRotator` 0.0 0.0 (/ `Speed Input` 0.1)) false false)
  (`SceneComponent.K2_AddLocalRotation` (`self.Wheel MR`) (`KismetMathLibrary.MakeRotator` 0.0 0.0 (/ `Speed Input` 0.1)) false false)
  (`SceneComponent.K2_AddLocalRotation` (`self.Wheel BR`) (`KismetMathLibrary.MakeRotator` 0.0 0.0 (/ `Speed Input` 0.1)) false false))

(fn `Calculate Turning`
  (params (`Action Value` :type "Float (double-precision)"))
  (bind _returnvalue (`PrimitiveComponent.GetMass` (`self.Box`)))
  (bind _returnvalue_2 (* `Action Value` (`self.Turning Speed`) _returnvalue 100.0))
  ; Applying the acceleration force to the wheels
  (`PrimitiveComponent.AddTorqueInRadians` (`self.Box`) (`KismetMathLibrary.MakeVector` 0.0 0.0 _returnvalue_2) "None" false)
  (`self.Calculate Right Track` (/ _returnvalue_2 100.0))
  (`self.Calculate Left track` (* (* (`local.Action Value`) -1.0) _returnvalue (/ (`self.Turning Speed`) 100.0) 100.0)))

(fn `CalculateAcceleration`
  (bind _accelerationinput (`self.AccelerationInput`))
  ; Calculates the Acceleration
  (bind _output_get (set `self.Acceleration` (* (`KismetMathLibrary.Lerp` 0.0 10.0 _accelerationinput) _accelerationinput)))
  (set `self.Acceleration` (`KismetMathLibrary.FInterpTo` (`self.AccelerationInput`) 0.0 (`GameplayStatics.GetWorldDeltaSeconds`) 0.3))
  (`self.Calculate Left track` _output_get)
  (`self.Calculate Right Track` _output_get))

(fn `Suspension Cast`
  (params (Wheelcomp :type "SceneComponent Object Reference"))
  (bind _box (`self.Box`))
  (for _array_element (`|MakeArray` (`self.FR Wheel`) (`self.FL Wheel`) (`self.BL Wheel`) (`self.BR Wheel`) (`self.ML Wheel`) (`self.MR Wheel`))
    (bind _returnvalue (`SceneComponent.K2_GetComponentLocation` _array_element))
    ; Calculates the suspension and its strength
    (bind _outhit (`KismetSystemLibrary.LineTraceSingle` :`Start` _returnvalue :`End` (* _returnvalue (* (`SceneComponent.GetUpVector` _array_element) -60.0)) :`TraceChannel` "TraceTypeQuery1" :`DrawDebugType` "ForOneFrame"))
    (bind (_bblockinghit _binitialoverlap _time _distance _location _impactpoint _normal _impactnormal _physmat _hitactor _hitcomponent _hitbonename _bonename _hititem _elementindex _faceindex _tracestart _traceend) (`GameplayStatics.BreakHitResult` _outhit))
    (if _bblockinghit
      (`PrimitiveComponent.AddForceAtLocation` (`self.Box`) (* (- 1.0 (`KismetMathLibrary.NormalizeToRange` _distance 0.0 60.0)) (`KismetMathLibrary.GetDirectionUnitVector` _traceend _tracestart) 50000.0) (`SceneComponent.K2_GetComponentLocation` _array_element) "None")
      ; Applying the acceleration force to the wheels
      (`PrimitiveComponent.AddForceAtLocation` (`self.Box`) (* (`SceneComponent.GetForwardVector` _box) 1000.0 (`self.Acceleration`) (`PrimitiveComponent.GetMass` _box)) (`SceneComponent.K2_GetComponentLocation` _array_element) "None")
      (bind _returnvalue_2 (`SceneComponent.GetChildComponent` _array_element 0))
      (bind (_relativelocation_x _relativelocation_y _relativelocation_z) (`KismetMathLibrary.BreakVector` (`SceneComponent.RelativeLocation` _returnvalue_2)))
      (`SceneComponent.K2_SetRelativeLocation` _returnvalue_2 (`KismetMathLibrary.MakeVector` 0.0 0.0 (`KismetMathLibrary.FInterpTo` _relativelocation_z (+ (* _distance -1.0) 30.0) (`GameplayStatics.GetWorldDeltaSeconds`) 3.0)) false false))))

(fn `UserConstructionScript`)